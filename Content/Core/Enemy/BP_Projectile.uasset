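; Enemy projectile that briefly homes on the player at spawn, then flies straight, with a per-tick Y offset step for shotgun-style shots.
; WorldDynamic overlap turns on after a short delay.
; Overlaps damage BPI_Damage actors and destroy the projectile, unless the player character is deflecting.
; Deflection swaps the sphere material and re-enables homing toward the owning BP_Cygnus's mesh, or destroys the projectile without a valid owner.
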(event Collision|EventActorBeginOverlap
  (params (OtherActor :type Actor%20Object%20Reference))
  (if true
    (bind _array_element (Utilities|Array|ForEachLoopwithBreak (Collision|GetOverlappingActors 0 :!class /Script/Engine.Actor))
      (:LoopBody
        (if (Utilities|DoesObjectImplementInterface _array_element "/Game/Core/Assets/Blueprints/BPI_Damage.BPI_Damage_C")
          (bind _asbp_my_2dcharacter (Utilities|Casting|CastToBP_My2DCharacter _array_element)
            (:then
              (if (Variables|/Game/Core/Character/BP_My2DCharacter.BP_My2DCharacter_C|GetisDeflecting _asbp_my_2dcharacter)
                (|DeflectBack)
                (else
                  (Class|BPIDamage|BPIDamage(Message) _array_element 1 :!label _label)
                  (Actor|DestroyActor))))
            (:CastFailed
              (goto _label))))))))

(event EventTick
  (params (DeltaSeconds :type Float%20%28single-precision%29))
  (bind _returnvalue (Transformation|GetActorTransform))
  (Transformation|SetActorTransform (Math|Transform|MakeTransform (Math|Vector|MakeVector (.x (.location _returnvalue)) (|AddOffSetToY(Shotgun) (.y (.location _returnvalue)) DeltaSeconds) (.z (.location _returnvalue))) (.rotation _returnvalue) (.scale _returnvalue))))

(event EventBeginPlay
  (Utilities|FlowControl|Sequence
    (:then_0
      (|SetVariables))
    (:then_1
      (|TowardsPlayer))
    (:then_2
      (Utilities|FlowControl|Delay 0.5)
      (Collision|SetCollisionResponsetoChannel (Variables|Default|GetSphere) "ECC_WorldDynamic" "ECR_Overlap"))))

(fn ConstructionScript)