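; BP_Cygnus is an enemy that faces the player and fires projectiles in short randomized bursts.
; A looping BeginPlay delay triggers bursts only while it sits within an X range.
; Tick shifts it along X relative to the GameInstance's Speed, destroys it far behind, and turns it toward the player.
; BPIDamage reduces Health and, on death, destroys it and awards drill to the player character.
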(event EventBeginPlay
  (bind _returnvalue (Transformation|GetActorLocation))
  (Utilities|FlowControl|Delay (Math|Random|RandomFloatinRange 1.5 3.0) :!label _label)
  (if (and (< (.x _returnvalue) 2.5e+04) (> (.x _returnvalue) 2e+03))
    (Variables|Default|SetTimes (Math|Random|RandomIntegerinRange 2 4))
    (Game|SpawnActorfromClass "/Game/Core/Enemy/BP_Projectile.BP_Projectile_C" (Math|Transform|MakeTransform (Math|Vector|MakeVector (.x _returnvalue) (.y _returnvalue) (.z _returnvalue)) "0, 0, 0" "1.000000,1.000000,1.000000") "Undefined" self 0 :!label _label_2)
    (if (> (Variables|Default|GetTimes) 0)
      (Utilities|FlowControl|Delay 0.05)
      (Variables|Default|SetTimes (- (Variables|Default|GetTimes) 1))
      (goto _label_2)
      (else
        (goto _label)))
    (else
      (goto _label))))

(event EventTick
  (params (DeltaSeconds :type Float%20%28single-precision%29))
  (bind _returnvalue (Transformation|GetActorLocation))
  (Utilities|FlowControl|Sequence
    (:then_0
      (bind _gameinstance (CallFunction|CasttoGameInstance))
      (if (!= (Variables|/Game/Core/Assets/Blueprints/BP_GameInstance.BP_GameInstance_C|GetSpeed _gameinstance) 0.0)
        (if (<= (.x _returnvalue) -3e+04)
          (Actor|DestroyActor)
          (else
            (Transformation|SetActorLocation (Math|Vector|MakeVector (- (.x _returnvalue) (* (- (Variables|/Game/Core/Assets/Blueprints/BP_GameInstance.BP_GameInstance_C|GetSpeed _gameinstance) 7e+03) DeltaSeconds)) (.y _returnvalue) (.z _returnvalue)) false false)))))
    (:then_1
      (|RotateTowardsPlayer DeltaSeconds))))

(event EventBPIDamage
  (params (Damage :type Integer))
  ;[1 1 1] Take Damage and Die event
  (Development|PrintString "Oof")
  (Variables|Default|SetHealth (- (Variables|Default|GetHealth) Damage))
  (if (<= (Variables|Default|GetHealth) 0.0)
    (Actor|DestroyActor)
    (bind _asbp_my_2dcharacter (Utilities|Casting|CastToBP_My2DCharacter (Game|GetPlayerCharacter 0)))
    (Default|BPIAddDrill _asbp_my_2dcharacter 2e+01)))

(fn ConstructionScript)

(fn BPIAddDrill
  (params (Amount :type Float%20%28double-precision%29)))