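; BP_ObstacleDestructable is an obstacle cube that loses a fixed amount of health on each hit and disappears when health runs out.
; Component hits decrement Health, and at zero the cube toggles visibility and disables collision instead of being destroyed.
; For testing, it prints health and reactivates after a short delay, restoring health, visibility and collision; component activation also triggers this reset.
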(event OnComponentActivated(Cube)
  (params (Component :type Actor%20Component%20Object%20Reference) (bReset :type Boolean))
  ;[1 1 1] Reactivate Obstacle
  (CallFunction|ReactivateObstacle))

(event OnComponentHit(Cube)
  (params (HitComponent :type Primitive%20Component%20Object%20Reference) (OtherActor :type Actor%20Object%20Reference) (OtherComp :type Primitive%20Component%20Object%20Reference) (NormalImpulse :type Vector :default "0, 0, 0") (Hit :type Hit%20Result%20Structure%20%28by%20ref%29))
  ;[1 1 1] Handle On Component Hit
  (CallFunction|DecrementHealth)
  ;[1 1 1] Testing Only
  (Development|PrintString (Utilities|String|ToString(Integer) (Variables|Default|GetHealth)))
  (if (<= (Variables|Default|GetHealth) 0)
    (CallFunction|HideObstacle)))

(event Custom|DecrementHealth
  ;[1 1 1] Decrease Health -> add int input that can be taken from caller
  (Variables|Default|SetHealth (- (Variables|Default|GetHealth) 10)))

(event Custom|HideObstacle
  ;[1 1 1] Hide Obstacle -> not visible, no collision
  (Rendering|ToggleVisibility (Variables|Default|GetCube) false)
  (Collision|SetCollisionEnabled (Variables|Default|GetCube) "NoCollision")
  ;[1 1 1] For Testing Only
  (Utilities|FlowControl|Delay 5.0)
  (CallFunction|ReactivateObstacle))

(event Custom|ReactivateObstacle
  ;[1 1 1] Reactivate Obstacle -> visible, has collision, reset health
  (Variables|Default|SetHealth 100)
  (Collision|SetCollisionEnabled (Variables|Default|GetCube) "QueryAndPhysics")
  (Rendering|SetVisibility (Variables|Default|GetCube) true false))

(fn ConstructionScript)