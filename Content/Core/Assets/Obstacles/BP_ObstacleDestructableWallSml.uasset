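; BP_ObstacleDestructableWallSml is a small destructible wall obstacle that loses a fixed amount of Health whenever BP_My2DCharacter begins overlapping its W component.
; When Health runs out, HideObstacle loops over the root's child components, turning off visibility and static mesh collision.
; A Delay inside that loop leads to ReactivateObstacle, which resets Health and restores visibility and collision.
; Debug prints report Health and hidden mesh names.
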(event OnComponentBeginOverlap(w)
  (params (OverlappedComponent :type Primitive%20Component%20Object%20Reference) (OtherActor :type Actor%20Object%20Reference) (OtherComp :type Primitive%20Component%20Object%20Reference) (OtherBodyIndex :type Integer) (bFromSweep :type Boolean) (SweepResult :type Hit%20Result%20Structure%20%28by%20ref%29))
  ;[1 1 1] Handle On Component Hit
  (Utilities|Casting|CastToBP_My2DCharacter OtherActor)
  (CallFunction|DecrementHealth)
  ;;[1 1 1] Testing Only
  (Development|PrintString (Utilities|String|ToString(Integer) (Variables|Default|GetHealth)))
  (if (<= (Variables|Default|GetHealth) 0)
    (CallFunction|HideObstacle)))

(event Custom|DecrementHealth
  ;[1 1 1] Decrease Health -> add int input that can be taken from caller
  (Variables|Default|SetHealth (- (Variables|Default|GetHealth) 10)))

(event Custom|HideObstacle
  (bind _defaultsceneroot (Variables|Default|GetDefaultSceneRoot))
  (bind _children (Components|GetChildrenComponents _defaultsceneroot false))
  ;[1 1 1] Hide Obstacle -> not visible, no collision
  (for (_array_element _array_index) _children
    (Rendering|SetVisibility _array_element false false)
    (bind _asstatic_mesh_component (Utilities|Casting|CastToStaticMeshComponent (Utilities|Array|Get(acopy) _children _array_index)))
    (Collision|SetCollisionEnabled _asstatic_mesh_component "NoCollision")
    ;[1 1 1] For Testing Only
    (Development|PrintString (Utilities|GetDisplayName _asstatic_mesh_component))
    (Utilities|FlowControl|Delay 5.0)
    (CallFunction|ReactivateObstacle)))

(event Custom|ReactivateObstacle
  (bind _defaultsceneroot (Variables|Default|GetDefaultSceneRoot))
  (bind _children (Components|GetChildrenComponents _defaultsceneroot false))
  ;[1 1 1] Reactivate Obstacle -> visible, has collision, reset health
  (Variables|Default|SetHealth 100)
  (for (_array_element _array_index) _children
    (Rendering|SetVisibility _array_element true false)
    (bind _asstatic_mesh_component (Utilities|Casting|CastToStaticMeshComponent (Utilities|Array|Get(acopy) _children _array_index)))
    (Collision|SetCollisionEnabled _asstatic_mesh_component "QueryAndPhysics")))

(fn ConstructionScript)