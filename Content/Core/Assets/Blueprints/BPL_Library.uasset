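; Blueprint function library of shared helpers for the 2D game, covering a global speed query and game instance access.
; ReturnSpeed reads the player character's drill state, giving zero while getting drilled and a fixed speed otherwise, with no explicit return during super drilling.
; CastToGameInstance returns the game instance cast to BP_GameInstance.
; ForEachLoopDelay is an unfinished stub whose loop nodes are disconnected from its entry.
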(fn ReturnSpeed
  (bind _asbp_my_2dcharacter (Utilities|Casting|CastToBP_My2DCharacter (Game|GetPlayerCharacter (LocalVariables|Get__WorldContext))))
  (LocalVariables|SetMy2DCharacter _asbp_my_2dcharacter)
  (if (not (Variables|/Game/Core/Character/BP_My2DCharacter.BP_My2DCharacter_C|GetisSuperDrilling (LocalVariables|GetMy2DCharacter)))
    (if (Variables|/Game/Core/Character/BP_My2DCharacter.BP_My2DCharacter_C|GetgettingDrilled (LocalVariables|GetMy2DCharacter))
      (LocalVariables|SetGlobalSpeed 0.0)
      (else
        (bind _output_get (LocalVariables|SetGlobalSpeed 75.0))))
    (return _output_get)))

(fn CasttoGameInstance
  (bind _asbp_game_instance (Utilities|Casting|CastToBP_GameInstance (Game|GetGameInstance (LocalVariables|Get__WorldContext))))
  (return _asbp_game_instance))

(fn ForEachLoopDelay
  (params (FirstIndex :type Integer) (LastIndex :type Integer) (Delay :type Float%20%28double-precision%29)))