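; BP_PoolingSystem is an early object-pool Blueprint that pre-spawns projectile actors when play begins.
; BeginPlay runs an indexed loop that spawns BP_Projectile at the Spawner's location, calls an array set at each index and prints each new actor's name.
; A matching BP_Cygnus loop is present but disconnected, so it never runs.
; The graph has no logic for retrieving or recycling pooled actors.
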(event EventBeginPlay
  (Utilities|FlowControl|Sequence
    (:then_1
      ;[1 1 1] Loops until we hit the given index
      (for _index (range 0 10)
        (bind _returnvalue (Game|SpawnActorfromClass "/Game/Core/Enemy/BP_Projectile.BP_Projectile_C" (Math|Transform|MakeTransform (Transformation|GetActorLocation (Variables|Default|GetSpawner)) "0, 0, 0" "1.000000,1.000000,1.000000") "Undefined" "OverrideRootScale" 0 0))
        ;[1 1 1] Sets array indexes until they are fulll
        (Utilities|Array|SetArrayElem (Utilities|Array|MakeArray 0) _index 0)
        (Development|PrintString (Utilities|GetDisplayName _returnvalue))))))