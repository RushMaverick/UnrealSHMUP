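; BP_ScrollingField drives an endless scrolling level by moving four referenced actors along negative X every Tick.
; Scroll speed comes from the Game Instance and is scaled by delta time.
; An actor passing the rear X threshold wraps ahead of its predecessor in the ring, offset by index parity, and triggers the wall and enemy spawners.
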(event EventBeginPlay)

(event EventTick
  (params (DeltaSeconds :type Float%20%28single-precision%29))
  (Variables|Default|SetDeltaS DeltaSeconds)
  (CallFunction|Speed (Utilities|Array|MakeArray (Variables|Components|GetActor1) (Variables|Components|GetActor2) (Variables|Components|GetActor3) (Variables|Components|GetActor4)) (Variables|Default|GetDeltaS)))

(fn ConstructionScript)

(fn Speed
  (params (ActorArray :type Array%20of%20Actor%20Object%20References) (Delta :type Float%20%28double-precision%29))
  (for (_array_element _array_index) ActorArray
    (bind _gameinstance (CallFunction|CasttoGameInstance))
    (if (<= (.x (Transformation|GetActorLocation _array_element)) -1.3e+03)
      (LocalVariables|SetArrayIndex _array_index)
      (if (> (Math|Integer|%(Integer) (LocalVariables|GetArrayIndex) 2) 0)
        (LocalVariables|SetNewLocalVar (+ (Transformation|GetActorLocation (Utilities|Array|Get(acopy) ActorArray (Math|Integer|%(Integer) (+ (LocalVariables|GetArrayIndex) 3) 4))) "3500.000000,0.000000,0.000000"))
        (else
          (LocalVariables|SetNewLocalVar (+ (Transformation|GetActorLocation (Utilities|Array|Get(acopy) ActorArray (Math|Integer|%(Integer) (+ (LocalVariables|GetArrayIndex) 3) 4))) "1700.000000,0.000000,0.000000"))))
      (Transformation|SetActorLocation _array_element (LocalVariables|GetNewLocalVar) false false)
      (Default|SpawnWall (Variables|Default|GetBP_Spawner))
      (Default|SpawnEnemy (Variables|Default|GetBP_SpawnerEnemy))
      (else
        (Transformation|SetActorLocation _array_element (Math|Vector|MakeVector (- (.x (Transformation|GetActorLocation _array_element)) (* (Variables|/Game/Core/Assets/Blueprints/BP_GameInstance.BP_GameInstance_C|GetSpeed _gameinstance) Delta)) (.y (Transformation|GetActorLocation _array_element)) (.z (Transformation|GetActorLocation _array_element))) false false)))))