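; Obstacle spawner that periodically places rows of BP_ObstacleDestructable at seven arrow points.
; Tick starts a randomized Delay, shorter when the game instance's Speed is high, then calls Spawn.
; Spawn randomizes per-point counts and picks lanes absent from LastIndex by random retry.
; Each chosen lane gets a column of obstacles stepped along X by looping back until its count reaches zero.
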(event Custom|Spawn
  (bind _arrayoftimes (Variables|Default|GetArrayOfTimes))
  (bind _spawnindex (Variables|Default|GetSpawnIndex))
  (bind _output (Utilities|Array|Get(acopy) _arrayoftimes _spawnindex))
  (|RandomizeArrayOfTimes
    (:Completed
      (for _index (range 0 (Variables|Default|GetLineSpawnN))
        (|SelectUniqueSpawnPoint
          (:OutputPin
            (Variables|Default|SetSpawnPoint (Transformation|GetWorldLocation (Utilities|Array|Get(acopy) (Utilities|Array|MakeArray (Variables|Default|GetArrow) (Variables|Default|GetArrow1) (Variables|Default|GetArrow2) (Variables|Default|GetArrow3) (Variables|Default|GetArrow4) (Variables|Default|GetArrow5) (Variables|Default|GetArrow6)) (Variables|Default|GetSpawnIndex))))
            (Utilities|Array|SetArrayElem (Variables|Default|GetLast%20Index) _index (Variables|Default|GetSpawnIndex) true)
            (Variables|Default|SetSpawnPoint (+ (Variables|Default|GetSpawnPoint) (Math|Vector|MakeVector 5e+02 0.0 0.0)) :!label _label)
            (Game|SpawnActorfromClass "/Game/Core/Assets/Obstacles/BP_ObstacleDestructable.BP_ObstacleDestructable_C" (Math|Transform|MakeTransform (Variables|Default|GetSpawnPoint) "0, 0, 0" "1.000000,1.000000,1.000000") "AdjustIfPossibleButDontSpawnIfColliding" 0 0)
            (if (> _output 0)
              (Utilities|Array|SetArrayElem (Variables|Default|GetArrayOfTimes) (Variables|Default|GetSpawnIndex) (- _output 1))
              (goto _label)))))
      (Variables|Default|SetisSpawning false))))

(event EventTick
  (params (DeltaSeconds :type Float%20%28single-precision%29))
  (bind _gameinstance (CallFunction|CasttoGameInstance))
  (if (or (not (Variables|Default|GetisSpawning)) (> (Variables|/Game/Core/Assets/Blueprints/BP_GameInstance.BP_GameInstance_C|GetSpeed _gameinstance) 2e+03))
    (Variables|Default|SetisSpawning true)
    (if (> (Variables|/Game/Core/Assets/Blueprints/BP_GameInstance.BP_GameInstance_C|GetSpeed _gameinstance) 2e+03)
      (Variables|Default|SetSpawnRate (Math|Random|RandomFloatinRange 1.0 1.5))
      (else
        (Variables|Default|SetSpawnRate (Math|Random|RandomFloatinRange 3.5 4.5))))
    (Utilities|FlowControl|Delay (Variables|Default|GetSpawnRate))
    (Variables|Default|SetLineSpawnN 1)
    (CallFunction|Spawn)))

(fn ConstructionScript)

(fn NewFunction)

(fn SPeed
  (params (actor :type Actor%20Object%20Reference))
  (bind _returnvalue (Transformation|GetActorLocation actor))
  (bind _returnvalue_2 (+ (.x _returnvalue) -1e+02))
  (if (<= _returnvalue_2 -1e+04)
    (Transformation|SetActorLocation "89660.000000,0.000000,-140.500000" false false)
    (else
      (Transformation|SetActorLocation (Math|Vector|MakeVector _returnvalue_2 (.y _returnvalue) (.z _returnvalue)) false false))))